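; Game instance for an idle game, holding money, item data, menu widgets and new/load start state across levels.
; Init copies the current quality tier's Data Table into an array.
; ItemsReadyToTick waits a second, then loops that array, accumulating exponential income, calling AddMoney and re-triggering itself per item.
; Show events lazily create cached UI-only menus; StartGame opens the level, and LevelLoaded has IdlePlayerController initialise new or saved data.
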(event Custom|AddMoney
  (params (Income :type Integer64))
  ;[1 1 1] Добавление денег
  (Variables|Default|SetAllMoney (+ Income (Variables|Default|GetAllMoney)))
  (Default|CallWhenMoneyAdd))

(event Custom|ItemsReadyToTick
  (params (Item%20Quality%20Type :type E_Item_Quality%20Enum :default "NewEnumerator0"))
  (bind _output_get (Variables|Default|SetItem%20Quality%20Type Item%20Quality%20Type))
  (switch Utilities|FlowControl|Switch|SwitchonE_Item_Quality _output_get
    (:NewEnumerator0
      (Variables|Default|SetCommonIncome 0)
      (Utilities|FlowControl|Delay 1.0)
      (for _array_element (Variables|Data|GetItemsData)
        (bind _output_get_2 (Variables|Default|SetCommonIncome (+ (Variables|Default|GetCommonIncome) (Class|KismetMathLibrary|FFloor64 (* (.Quantity (Utilities|Struct|Break1X_ItemData _array_element)) (Math|Float|Power 1.2 (.Income (Utilities|Struct|Break1X_ItemData _array_element))))))))
        (CallFunction|AddMoney _output_get_2)
        (CallFunction|ItemsReadytoTick (Variables|Default|GetItem%20Quality%20Type))))
    (:NewEnumerator1
      (Variables|Default|SetCommonIncome 0)
      (Utilities|FlowControl|Delay 1.0)
      (for _array_element_2 (Variables|Data|Get2X_Item_Data)
        (bind _output_get_3 (Variables|Default|SetCommonIncome (+ (Variables|Default|GetCommonIncome) (Class|KismetMathLibrary|FFloor64 (* (.Quantity (Utilities|Struct|Break2X_Item_Data _array_element_2)) (Math|Float|Power 1.2 (.Income (Utilities|Struct|Break2X_Item_Data _array_element_2))))))))
        (CallFunction|AddMoney _output_get_3)
        (CallFunction|ItemsReadytoTick (Variables|Default|GetItem%20Quality%20Type))))
    (:NewEnumerator2
      (Variables|Default|SetCommonIncome 0)
      (Utilities|FlowControl|Delay 1.0)
      (for _array_element_3 (Variables|Data|Get3X_Item_Data)
        (bind _output_get_4 (Variables|Default|SetCommonIncome (+ (Variables|Default|GetCommonIncome) (Class|KismetMathLibrary|FFloor64 (* (.Quantity (Utilities|Struct|Break3X_Item_Data _array_element_3)) (Math|Float|Power 1.2 (.Income (Utilities|Struct|Break3X_Item_Data _array_element_3))))))))
        (CallFunction|AddMoney _output_get_4)
        (CallFunction|ItemsReadytoTick (Variables|Default|GetItem%20Quality%20Type))))))

(event Custom|Show%20Skins%20Menu
  (bind _returnvalue (Game|GetPlayerController 0))
  ;[1 1 1] Вызов Меню Скинов
  (Utilities|IsValid (Variables|Widgets|GetUI%20Skins%20Menu%20WB)
    (:Is%20Valid
      _)
    (:Is%20Not%20Valid
      (bind _returnvalue_2 (UserInterface|CreateWidget "/Game/UI/Minor_Menus/UI_Skins.UI_Skins_C" _returnvalue))
      (Variables|Widgets|SetUI%20Skins%20Menu%20WB _returnvalue_2)))
  (UserInterface|Viewport|AddtoViewport (Variables|Widgets|GetUI%20Skins%20Menu%20WB) 0)
  (Variables|/Script/Engine.PlayerController|SetbShowMouseCursor _returnvalue true)
  (Input|SetInputModeUIOnly _returnvalue (Variables|Widgets|GetUI%20Skins%20Menu%20WB) "DoNotLock"))

(event Custom|Create%20New%20game
  ;[1 1 1] Начало Новой Игры
  (Input|SetInputModeGameOnly (Game|GetPlayerController 0))
  (Game|OpenLevel(byName) "StartLevel"))

(event Custom|Start%20Game
  (params (Start%20Game%20Type :type E_Init_Type%20Enum :default "NewEnumerator0") (GamePlay%20Data%20%28if%20we%20loaded%20game%29 :type Gameplay%20Save%20Data%20Structure%20Structure))
  ;[1 1 1] Старт игры
  (bind _output_get (Variables|Default|SetStart%20Game%20Type Start%20Game%20Type))
  (switch Utilities|FlowControl|Switch|SwitchonE_Init_Type _output_get
    (:NewEnumerator0
      (CallFunction|CreateNewGame))
    (:NewEnumerator1
      (CallFunction|LoadSavedGame GamePlay%20Data%20%28if%20we%20loaded%20game%29))))

(event Custom|Load%20Saved%20Game
  (params (GamePlay%20Data :type Gameplay%20Save%20Data%20Structure%20Structure))
  (bind _returnvalue (Game|GetPlayerController 0))
  ;[1 1 1] Старт игры из загрузки
  (Variables|Default|Setgameplay%20Data%20For%20load GamePlay%20Data)
  (Variables|/Script/Engine.PlayerController|SetbShowMouseCursor _returnvalue false)
  (Input|SetInputModeGameOnly _returnvalue)
  (Viewport|RemoveAllWidgets)
  (Utilities|FlowControl|Delay 2.0) ; Можно без делея
  (Game|OpenLevel(byName) "Start Level"))

(event Custom|Level%20Loaded
  ;[1 1 1] Логика загрузки игры
  (switch Utilities|FlowControl|Switch|SwitchonE_Init_Type (Variables|Default|GetStart%20Game%20Type)
    (:NewEnumerator0
      (Default|InitNewGame (.AsIdle%20Player%20Controller (Utilities|Casting|CastToIdlePlayerController (Game|GetPlayerController 0)))))
    (:NewEnumerator1
      (Default|InitSavedGame (.AsIdle%20Player%20Controller (Utilities|Casting|CastToIdlePlayerController (Game|GetPlayerController 0))) (Variables|Default|Getgameplay%20Data%20For%20load)))))

(event Custom|Show%20Settings%20Menu
  (bind _returnvalue (Game|GetPlayerController 0))
  ;[1 1 1] Вызов Меню Настроек
  (Utilities|IsValid (Variables|Widgets|GetUI%20Settings%20Menu%20WB)
    (:Is%20Valid
      _)
    (:Is%20Not%20Valid
      (bind _returnvalue_2 (UserInterface|CreateWidget "/Game/UI/Minor_Menus/UI_Settings.UI_Settings_C" _returnvalue))
      (Variables|Widgets|SetUI%20Settings%20Menu%20WB _returnvalue_2)))
  (UserInterface|Viewport|AddtoViewport (Variables|Widgets|GetUI%20Settings%20Menu%20WB) 0)
  (Variables|/Script/Engine.PlayerController|SetbShowMouseCursor _returnvalue true)
  (Input|SetInputModeUIOnly _returnvalue (Variables|Widgets|GetUI%20Settings%20Menu%20WB) "DoNotLock"))

(event Custom|Show%20UI%20test
  (bind _returnvalue (Game|GetPlayerController 0))
  (Utilities|IsValid (Variables|Default|Gettest1)
    (:Is%20Valid
      _)
    (:Is%20Not%20Valid
      (bind _returnvalue_2 (UserInterface|CreateWidget "/Game/UI/Minor_Menus/test.test_C" _returnvalue))
      (Variables|Default|Settest1 _returnvalue_2)))
  (UserInterface|Viewport|AddtoViewport (Variables|Default|Gettest1) 0)
  (Variables|/Script/Engine.PlayerController|SetbShowMouseCursor _returnvalue true)
  (Input|SetInputModeUIOnly _returnvalue (Variables|Default|Gettest1) "DoNotLock"))

(event Custom|Show%20Main%20Menu
  (bind _returnvalue (Game|GetPlayerController 0))
  ;[1 1 1] Вызов главного меню
  (Utilities|IsValid (Variables|Widgets|GetUI%20Idle%20Main%20Menu%20WB)
    (:Is%20Valid
      _)
    (:Is%20Not%20Valid
      (bind _returnvalue_2 (UserInterface|CreateWidget "/Game/UI/UI_IdleMain.UI_IdleMain_C" _returnvalue))
      (Variables|Widgets|SetUI%20Idle%20Main%20Menu%20WB _returnvalue_2)))
  (UserInterface|Viewport|AddtoViewport (Variables|Widgets|GetUI%20Idle%20Main%20Menu%20WB) 0)
  (Variables|/Script/Engine.PlayerController|SetbShowMouseCursor _returnvalue true)
  (Input|SetInputModeUIOnly _returnvalue (Variables|Widgets|GetUI%20Idle%20Main%20Menu%20WB) "DoNotLock"))

(event Custom|Show%20Market%20Menu
  (bind _returnvalue (Game|GetPlayerController 0))
  ;[1 1 1] Вызов Меню Магазина
  (Utilities|IsValid (Variables|Widgets|GetUI%20Market%20Menu%20WB)
    (:Is%20Valid
      _)
    (:Is%20Not%20Valid
      (bind _returnvalue_2 (UserInterface|CreateWidget "/Game/UI/Minor_Menus/UI_Market.UI_Market_C" _returnvalue))
      (Variables|Widgets|SetUI%20Market%20Menu%20WB _returnvalue_2)))
  (UserInterface|Viewport|AddtoViewport (Variables|Widgets|GetUI%20Market%20Menu%20WB) 0)
  (Variables|/Script/Engine.PlayerController|SetbShowMouseCursor _returnvalue true)
  (Input|SetInputModeUIOnly _returnvalue (Variables|Widgets|GetUI%20Market%20Menu%20WB) "DoNotLock"))

(event Custom|Show%20Buy%20Menu
  (bind _returnvalue (Game|GetPlayerController 0))
  ;[1 1 1] Вызов Меню Улучшения
  (Utilities|IsValid (Variables|Widgets|GetUI%20Buy%20Menu%20WB)
    (:Is%20Valid
      _)
    (:Is%20Not%20Valid
      (bind _returnvalue_2 (UserInterface|CreateWidget "/Game/UI/Minor_Menus/UI_menu.UI_menu_C" _returnvalue))
      (Variables|Widgets|SetUI%20Buy%20Menu%20WB _returnvalue_2)))
  (UserInterface|Viewport|AddtoViewport (Variables|Widgets|GetUI%20Buy%20Menu%20WB) 0)
  (Variables|/Script/Engine.PlayerController|SetbShowMouseCursor _returnvalue true)
  (Input|SetInputModeUIOnly _returnvalue (Variables|Widgets|GetUI%20Buy%20Menu%20WB) "DoNotLock"))

(event EventInit
  ;[1 1 1] Перевод Data Table в массив
  (switch Utilities|FlowControl|Switch|SwitchonE_Item_Quality (Variables|Default|GetItem%20Quality%20Type)
    (:NewEnumerator0
      (bind _outrownames (DataTable|GetDataTableRowNames "/Game/Data/DataTables/1X_Items.1X_Items"))
      (for _array_element _outrownames
        (bind _returnvalue (Utilities|GetDataTableRow "/Game/Data/DataTables/1X_Items.1X_Items" _array_element)
          (:then
            (Utilities|Array|Add (Variables|Data|GetItemsData) _returnvalue)))))
    (:NewEnumerator1
      (bind _outrownames_2 (DataTable|GetDataTableRowNames "/Game/Data/DataTables/2X_Items.2X_Items"))
      (for _array_element_2 _outrownames_2
        (bind _returnvalue_2 (Utilities|GetDataTableRow "/Game/Data/DataTables/2X_Items.2X_Items" _array_element_2)
          (:then
            (Utilities|Array|Add (Variables|Data|Get2X_Item_Data) _returnvalue_2)))))
    (:NewEnumerator2
      (bind _outrownames_3 (DataTable|GetDataTableRowNames "/Game/Data/DataTables/3X_Items.3X_Items"))
      (for _array_element_3 _outrownames_3
        (bind _returnvalue_3 (Utilities|GetDataTableRow "/Game/Data/DataTables/3X_Items.3X_Items" _array_element_3)
          (:then
            (Utilities|Array|Add (Variables|Data|Get3X_Item_Data) _returnvalue_3)))))))