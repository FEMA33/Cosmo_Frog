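; Player controller for an idle game, meant to spawn and possess the IdleCharacter for a new or saved game.
; All events are empty; their apparent logic sits in disconnected chains that never run.
; Those chains cache the GI_Idle game instance and report level load, then spawn at the first PlayerStart with zero money or at the saved transform with saved money.
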(event Custom|Init%20New%20Game
  ;[1 1 1] Инит Новой игры
)

(event Custom|Init%20Saved%20Game
  (params (Gameplay :type Gameplay%20Save%20Data%20Structure%20Structure)))

(event EventBeginPlay
  ;[1 1 1] Записываем в переменную ссылку на гейм инст
)

(event EventPossess
  (params (PossessedPawn :type Pawn%20Object%20Reference)))

(fn ConstructionScript)